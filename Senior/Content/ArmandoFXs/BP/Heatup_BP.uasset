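; Heat-up effect Blueprint that reacts to the blue potion state of a cauldron.
; On every Tick it casts CauldronC to Cauldron_BP and, while PotionBlue is set, spawns the C_Effect_2 emitter attached at Test1, with no guard against repeat spawns.
; IncrementCounter bumps a counter, CheckSolution always returns false, and HeatUp, ResetFlags and ChangeColor are empty stubs.
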(event EventTick
  (params (DeltaSeconds :type Float%20%28single-precision%29))
  (bind _ascauldron_bp (Utilities|Casting|CastToCauldron_BP (Variables|Default|GetCauldron_C)))
  (if (Variables|/Game/ArmandoFXs/BP/Cauldron_BP.Cauldron_BP_C|GetpotionBlue _ascauldron_bp)
    (Effects|SpawnEmitterAttached "/Game/ArmandoFXs/C_Effect_2.C_Effect_2" 0 "None" (Transformation|GetSocketLocation (Variables|Default|Gettest1) "None"))))

(fn ConstructionScript)

(fn CheckSolution
  (return false))

(fn ResetFlags
  (params (Cauldron :type Cauldron%20BP%20Object%20Reference)))

(fn ChangeColor)

(fn IncrementCounter
  (bind _result (Math|Integer|IncrementInt (Variables|Default|GetCounter))))

(fn HeatUp)