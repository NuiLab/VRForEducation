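; Cauldron Blueprint that accepts red and blue potions and plays staged brewing effects.
; On overlap, it matches the actor's display name to flag potions as added, then destroys any actor not named as the player.
; HeatUp, not called within this Blueprint, requires both flags: its first stage spawns an emitter at CEffect, clears them and advances a counter.
; The second stage spawns another effect without advancing; the third is empty.
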(event Collision|EventActorBeginOverlap
  (params (OtherActor :type Actor%20Object%20Reference))
  (CallFunction|CheckObject OtherActor)
  (CallFunction|FlagPotion (Utilities|GetDisplayName OtherActor))
  (CallFunction|DeleteObject OtherActor))

(fn ConstructionScript)

(fn CheckObject
  (params (NewParam :type Actor%20Object%20Reference))
  (bind _returnvalue (Utilities|GetDisplayName NewParam))
  (bind _returnvalue_2 (Utilities|Text|ToText(String) _returnvalue))
  (bind _returnvalue_3 (Utilities|String|ToString(Text) _returnvalue_2))
  (if (Utilities|Enum|Equal(Enum) (Variables|Default|GetpBlue) _returnvalue_3)
    (if (not (Variables|Default|GetpotionBlue))
      (CallFunction|FlagPotion (Variables|Default|GetpBlue)))
    (elif (Utilities|Enum|Equal(Enum) (Variables|Default|GetpRed) _returnvalue_3)
      (if (not (Variables|Default|GetpotionRed))
        (CallFunction|FlagPotion (Variables|Default|GetpRed))))))

(fn FlagPotion
  (params (potion :type String))
  (if (Utilities|Enum|Equal(Enum) potion (Variables|Default|GetpBlue))
    (Variables|Default|SetpotionBlue true)
    (elif (Utilities|Enum|Equal(Enum) potion (Variables|Default|GetpRed))
      (Variables|Default|SetpotionRed true))))

(fn DeleteObject
  (params (NewParam :type Actor%20Object%20Reference))
  (if (not (Utilities|Enum|Equal(Enum) (Variables|Default|Getplayer) (Utilities|GetDisplayName NewParam)))
    (Actor|DestroyActor NewParam)))

(fn ErrorMsg)

(fn HeatUp
  (bind _c_effect (Variables|Default|GetC_Effect))
  (bind _returnvalue (Transformation|GetSocketLocation _c_effect "None"))
  (if (Variables|Default|GetpotionRed)
    (if (Variables|Default|GetpotionBlue)
      (if (== 0 (Variables|Default|Getcounter))
        (bind _result (Math|Integer|IncrementInt (Variables|Default|Getcounter))
          (:%20%20
            (Variables|Default|Setcounter _result)
            (Variables|Default|SetpotionRed false)
            (Variables|Default|SetpotionBlue false)
            (Effects|SpawnEmitteratLocation "/Game/ArmandoFXs/C_Effect_1.C_Effect_1" _returnvalue "0, 0, 0" "1.000000,1.000000,1.000000" false)))
        (elif (== 1 (Variables|Default|Getcounter))
          (Effects|SpawnEmitteratLocation "/Game/ArmandoFXs/C_Effect_2.C_Effect_2" _returnvalue)
          (elif (== 2 (Variables|Default|Getcounter))
            _))))))