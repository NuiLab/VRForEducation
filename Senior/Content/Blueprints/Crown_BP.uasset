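; Crown_BP is an actor that makes a crown and its pillow float.
; At BeginPlay it records the starting world locations of the Crown and Pillow components, then plays a timeline.
; Each timeline update adds the Floating track value to both stored locations, so the two pieces move together as offsets from where they started.
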(event EventBeginPlay
  (Utilities|FlowControl|Sequence
    (:then_0
      (Variables|Default|SetInitialCrown (Transformation|GetWorldLocation (Variables|Default|GetCrown))))
    (:then_1
      (Variables|Default|SetInitialPillow (Transformation|GetWorldLocation (Variables|Default|GetPillow)))
      (bind _floating (Timeline|Timeline Play)
        (:Update
          (Utilities|FlowControl|Sequence
            (:then_1
              (Transformation|SetWorldLocation (Variables|Default|GetCrown) (+ _floating (Variables|Default|GetInitialCrown)) false false))
            (:then_2
              (Transformation|SetWorldLocation (Variables|Default|GetPillow) (+ _floating (Variables|Default|GetInitialPillow)) false false))))))))

(fn ConstructionScript)