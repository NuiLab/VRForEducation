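; Trigger actor that marks the player's entry into the IF room, firing once when Player_BP overlaps it.
; A Flag gate blocks repeat triggers, then the first Get_Metrics_BP found logs the room entry to its Metrics.
; It also calls NextLevel, shows the INTRO_IF widget and sets the level counter on the HUD_BP widget to the first of three.
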(event Collision|EventActorBeginOverlap
  (params (OtherActor :type Actor%20Object%20Reference))
  (Utilities|Casting|CastToPlayer_BP OtherActor)
  (if (Variables|Default|GetFlag)
    (Variables|Default|SetFlag false)
    (bind _outactors (Actor|GetAllActorsOfClass "/Game/Blueprints/Get_Metrics_BP.Get_Metrics_BP_C"))
    (Class|Metrics|EnteredRoom (Variables|/Game/Blueprints/Get_Metrics_BP.Get_Metrics_BP_C|GetMetrics (Utilities|Array|Get(acopy) _outactors)) "IF")
    (Default|CallNextLevel 1)
    (bind _returnvalue (UserInterface|CreateWidget "/Game/Blueprints/INTRO_IF.INTRO_IF_C"))
    (UserInterface|Viewport|AddtoViewport _returnvalue 0)
    (bind _foundwidgets (Widget|GetAllWidgetsOfClass "/Game/Blueprints/HUD_BP.HUD_BP_C" true))
    (Variables|/Game/Blueprints/HUD_BP.HUD_BP_C|SetCurrentLevel (Utilities|Array|Get(acopy) _foundwidgets) "1 / 3")))

(fn ConstructionScript)