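; If_Door_BP is a double door for the "IF" puzzle that swings open and closed on RoomOneDoor open and close events.
; A timeline yaws both leaves relative to their starting rotations and reverses on close.
; Its Sound Timing track plays the lock sound and, once via AchievementFlag, shows the IF achievement widget, briefly flags it on Player_BP and reports the solve to Get_Metrics_BP.
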(event OnOpen(RoomOneDoor)
  (bind (_direction _leftangle _rightangle) (Timeline|Timeline Play)
    (:Update
      (Utilities|FlowControl|Sequence
        (:then_0
          (Transformation|SetWorldRotation (Variables|Default|GetLeftDoor) (Math|Rotator|CombineRotators (Math|Rotator|MakeRotator 0.0 0.0 _leftangle) (Variables|Default|GetInitial%20Left)) false false))
        (:then_1
          (Transformation|SetWorldRotation (Variables|Default|GetRigthDoor) (Math|Rotator|CombineRotators (Math|Rotator|MakeRotator 0.0 0.0 _rightangle) (Variables|Default|GetInitial%20Right)) false false))))
    (:Sound%20Timing
      (Audio|PlaySoundatLocation "/Game/Audio/door-lock.door-lock" (Transformation|GetActorLocation))
      (if (Variables|Default|GetAchievementFlag)
        (Variables|Default|SetAchievementFlag false)
        (Utilities|FlowControl|Sequence
          (:then_0
            (bind _returnvalue (UserInterface|CreateWidget "/Game/Blueprints/ACHV_IF.ACHV_IF_C"))
            (UserInterface|Viewport|AddtoViewport _returnvalue 0)
            (bind _outactors (Actor|GetAllActorsOfClass "/Game/ThirdPersonBP/Blueprints/Player_BP.Player_BP_C"))
            (Utilities|FlowControl|Sequence
              (:then_0
                (Variables|/Game/ThirdPersonBP/Blueprints/Player_BP.Player_BP_C|SetShowACHV (Utilities|Array|Get(acopy) _outactors) true)
                (Utilities|FlowControl|Delay 4.0)
                (Variables|/Game/ThirdPersonBP/Blueprints/Player_BP.Player_BP_C|SetShowACHV (Utilities|Array|Get(acopy) _outactors) false))
              (:then_1
                (Variables|/Game/ThirdPersonBP/Blueprints/Player_BP.Player_BP_C|SetCurrent_ACHV (Utilities|Array|Get(acopy) _outactors) "IF"))))
          (:then_1
            (bind _outactors_2 (Actor|GetAllActorsOfClass "/Game/Blueprints/Get_Metrics_BP.Get_Metrics_BP_C"))
            (Class|Metrics|PuzzleSolved (Variables|/Game/Blueprints/Get_Metrics_BP.Get_Metrics_BP_C|GetMetrics (Utilities|Array|Get(acopy) _outactors_2)) "IF")))))))

(event OnClose(RoomOneDoor)
  (bind (_direction _leftangle _rightangle) (Timeline|Timeline Reverse)
    (:Update
      (Utilities|FlowControl|Sequence
        (:then_0
          (Transformation|SetWorldRotation (Variables|Default|GetLeftDoor) (Math|Rotator|CombineRotators (Math|Rotator|MakeRotator 0.0 0.0 _leftangle) (Variables|Default|GetInitial%20Left)) false false))
        (:then_1
          (Transformation|SetWorldRotation (Variables|Default|GetRigthDoor) (Math|Rotator|CombineRotators (Math|Rotator|MakeRotator 0.0 0.0 _rightangle) (Variables|Default|GetInitial%20Right)) false false))))
    (:Sound%20Timing
      (Audio|PlaySoundatLocation "/Game/Audio/door-lock.door-lock" (Transformation|GetActorLocation))
      (if (Variables|Default|GetAchievementFlag)
        (Variables|Default|SetAchievementFlag false)
        (Utilities|FlowControl|Sequence
          (:then_0
            (bind _returnvalue (UserInterface|CreateWidget "/Game/Blueprints/ACHV_IF.ACHV_IF_C"))
            (UserInterface|Viewport|AddtoViewport _returnvalue 0)
            (bind _outactors (Actor|GetAllActorsOfClass "/Game/ThirdPersonBP/Blueprints/Player_BP.Player_BP_C"))
            (Utilities|FlowControl|Sequence
              (:then_0
                (Variables|/Game/ThirdPersonBP/Blueprints/Player_BP.Player_BP_C|SetShowACHV (Utilities|Array|Get(acopy) _outactors) true)
                (Utilities|FlowControl|Delay 4.0)
                (Variables|/Game/ThirdPersonBP/Blueprints/Player_BP.Player_BP_C|SetShowACHV (Utilities|Array|Get(acopy) _outactors) false))
              (:then_1
                (Variables|/Game/ThirdPersonBP/Blueprints/Player_BP.Player_BP_C|SetCurrent_ACHV (Utilities|Array|Get(acopy) _outactors) "IF"))))
          (:then_1
            (bind _outactors_2 (Actor|GetAllActorsOfClass "/Game/Blueprints/Get_Metrics_BP.Get_Metrics_BP_C"))
            (Class|Metrics|PuzzleSolved (Variables|/Game/Blueprints/Get_Metrics_BP.Get_Metrics_BP_C|GetMetrics (Utilities|Array|Get(acopy) _outactors_2)) "IF")))))))

(event EventBeginPlay
  (Utilities|FlowControl|Sequence
    (:then_0
      (Variables|Default|SetInitial%20Left (Transformation|GetWorldRotation (Variables|Default|GetLeftDoor))))
    (:then_1
      (Variables|Default|SetInitial%20Right (Transformation|GetWorldRotation (Variables|Default|GetRigthDoor))))))

(fn ConstructionScript)