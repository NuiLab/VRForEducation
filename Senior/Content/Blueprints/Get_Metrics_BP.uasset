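; Get_Metrics_BP is an overlap-triggered actor that ends the game when Player_BP touches it.
; A Flag check clears itself on the first pass, then the actor calls EndGame on Metrics.
; After a three-second delay it pauses the game, shows the mouse cursor and opens the CreditsAch widget with focused game-and-UI input.
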(event Collision|EventActorBeginOverlap
  (params (OtherActor :type Actor%20Object%20Reference))
  (bind _returnvalue (Game|GetPlayerController 0))
  (Utilities|Casting|CastToPlayer_BP OtherActor)
  (if (Variables|Default|GetFlag)
    (Variables|Default|SetFlag false)
    (Class|Metrics|EndGame (Variables|Default|GetMetrics))
    (Utilities|FlowControl|Delay 3.0)
    (Game|SetGamePaused true)
    (Variables|/Script/Engine.PlayerController|SetbShowMouseCursor _returnvalue true)
    (bind _returnvalue_2 (UserInterface|CreateWidget "/Game/Blueprints/CreditsAch.CreditsAch_C" _returnvalue))
    (UserInterface|Viewport|AddtoViewport _returnvalue_2 0)
    (Input|SetInputModeGameandUI _returnvalue _returnvalue_2 "DoNotLock" false)))

(fn ConstructionScript)