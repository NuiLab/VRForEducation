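; A double door for the ARR puzzle that swings open and closed on the OpenDoor OnOpen and OnClose events.
; A timeline yaws both leaves relative to rotations cached at BeginPlay and reverses to close.
; Its Sound Timing event plays the lock sound and, gated by a one-shot AchievementFlag, shows the ACHV_ARR achievement widget and reports the solved puzzle to the player's Metrics.
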(event OnOpen(OpenDoor)
  (bind (_direction _leftangle _rightangle) (Timeline|Timeline_0 Play)
    (:Update
      (Utilities|FlowControl|Sequence
        (:then_0
          (Transformation|SetWorldRotation (Variables|Default|GetLeftDoor) (Math|Rotator|CombineRotators (Math|Rotator|MakeRotator 0.0 0.0 _leftangle) (Variables|Default|GetInitial%20Left)) false false))
        (:then_1
          (Transformation|SetWorldRotation (Variables|Default|GetRightDoor) (Math|Rotator|CombineRotators (Math|Rotator|MakeRotator 0.0 0.0 _rightangle) (Variables|Default|GetInitial%20Right)) false false))))
    (:Sound%20Timing
      (Audio|PlaySoundatLocation "/Game/Audio/door-lock.door-lock" (Transformation|GetActorLocation))
      (if (Variables|Default|GetAchievementFlag)
        (Variables|Default|SetAchievementFlag false)
        (Utilities|FlowControl|Sequence
          (:then_0
            (bind _returnvalue (UserInterface|CreateWidget "/Game/Blueprints/ACHV_ARR.ACHV_ARR_C"))
            (UserInterface|Viewport|AddtoViewport _returnvalue 0))
          (:then_1
            (bind _outactors (Actor|GetAllActorsOfClass "/Game/ThirdPersonBP/Blueprints/Player_BP.Player_BP_C"))
            (Class|Metrics|PuzzleSolved (Variables|/Game/ThirdPersonBP/Blueprints/Player_BP.Player_BP_C|GetMetrics (Utilities|Array|Get(acopy) _outactors)) "ARR")))))))

(event OnClose(OpenDoor)
  (bind (_direction _leftangle _rightangle) (Timeline|Timeline_0 Reverse)
    (:Update
      (Utilities|FlowControl|Sequence
        (:then_0
          (Transformation|SetWorldRotation (Variables|Default|GetLeftDoor) (Math|Rotator|CombineRotators (Math|Rotator|MakeRotator 0.0 0.0 _leftangle) (Variables|Default|GetInitial%20Left)) false false))
        (:then_1
          (Transformation|SetWorldRotation (Variables|Default|GetRightDoor) (Math|Rotator|CombineRotators (Math|Rotator|MakeRotator 0.0 0.0 _rightangle) (Variables|Default|GetInitial%20Right)) false false))))
    (:Sound%20Timing
      (Audio|PlaySoundatLocation "/Game/Audio/door-lock.door-lock" (Transformation|GetActorLocation))
      (if (Variables|Default|GetAchievementFlag)
        (Variables|Default|SetAchievementFlag false)
        (Utilities|FlowControl|Sequence
          (:then_0
            (bind _returnvalue (UserInterface|CreateWidget "/Game/Blueprints/ACHV_ARR.ACHV_ARR_C"))
            (UserInterface|Viewport|AddtoViewport _returnvalue 0))
          (:then_1
            (bind _outactors (Actor|GetAllActorsOfClass "/Game/ThirdPersonBP/Blueprints/Player_BP.Player_BP_C"))
            (Class|Metrics|PuzzleSolved (Variables|/Game/ThirdPersonBP/Blueprints/Player_BP.Player_BP_C|GetMetrics (Utilities|Array|Get(acopy) _outactors)) "ARR")))))))

(event EventBeginPlay
  (Utilities|FlowControl|Sequence
    (:then_0
      (Variables|Default|SetInitial%20Left (Transformation|GetWorldRotation (Variables|Default|GetLeftDoor))))
    (:then_1
      (Variables|Default|SetInitial%20Right (Transformation|GetWorldRotation (Variables|Default|GetRightDoor))))))

(fn ConstructionScript)