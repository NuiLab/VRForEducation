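; Double door Blueprint that swings two leaves open and closed and plays a door lock sound.
; BeginPlay caches each leaf's world rotation, and a timeline supplies separate left and right yaw angles that are combined with those cached rotations.
; OnOpen_Event plays the timeline and OnClose_Event reverses it, while a timeline event track times the sound at the actor's location.
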(event Custom|OnOpen_Event
  (bind (_direction _leftangle _rightangle) (Timeline|Timeline Play)
    (:Update
      (Utilities|FlowControl|Sequence
        (:then_0
          (Transformation|SetWorldRotation (Variables|Default|GetLeftDoor) (Math|Rotator|CombineRotators (Math|Rotator|MakeRotator 0.0 0.0 _leftangle) (Variables|Default|GetInitial%20Left)) false false))
        (:then_1
          (Transformation|SetWorldRotation (Variables|Default|GetRigthDoor) (Math|Rotator|CombineRotators (Math|Rotator|MakeRotator 0.0 0.0 _rightangle) (Variables|Default|GetInitial%20Right)) false false))))
    (:Sound%20Timing
      (Audio|PlaySoundatLocation "/Game/Audio/door-lock.door-lock" (Transformation|GetActorLocation)))))

(event Custom|OnClose_Event
  (bind (_direction _leftangle _rightangle) (Timeline|Timeline Reverse)
    (:Update
      (Utilities|FlowControl|Sequence
        (:then_0
          (Transformation|SetWorldRotation (Variables|Default|GetLeftDoor) (Math|Rotator|CombineRotators (Math|Rotator|MakeRotator 0.0 0.0 _leftangle) (Variables|Default|GetInitial%20Left)) false false))
        (:then_1
          (Transformation|SetWorldRotation (Variables|Default|GetRigthDoor) (Math|Rotator|CombineRotators (Math|Rotator|MakeRotator 0.0 0.0 _rightangle) (Variables|Default|GetInitial%20Right)) false false))))
    (:Sound%20Timing
      (Audio|PlaySoundatLocation "/Game/Audio/door-lock.door-lock" (Transformation|GetActorLocation)))))

(event EventBeginPlay
  (Utilities|FlowControl|Sequence
    (:then_0
      (Variables|Default|SetInitial%20Left (Transformation|GetWorldRotation (Variables|Default|GetLeftDoor))))
    (:then_1
      (Variables|Default|SetInitial%20Right (Transformation|GetWorldRotation (Variables|Default|GetRigthDoor))))))

(fn ConstructionScript)