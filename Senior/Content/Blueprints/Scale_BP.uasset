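; Scale Blueprint that animates a two-plate balance in response to the MagicScale event from ScaleWeightDisplayer.
; BeginPlay caches each plate's world location as its rest position.
; MagicScale passes left and right height offsets and restarts a timeline that moves both plates toward rest plus offset.
; Each update lerps from the plate's current location, so the easing compounds rather than following the timeline curve directly.
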(event MagicScale(ScaleWeightDisplayer)
  (params (LeftHeight :type Vector :default "0, 0, 0") (RightHeight :type Vector :default "0, 0, 0"))
  (bind _move_to (Timeline|Timeline PlayFromStart)
    (:Update
      (Utilities|FlowControl|Sequence
        (:then_0
          (Transformation|SetWorldLocation (Variables|Default|GetLeftPlate) (Math|Vector|Lerp(Vector) (Transformation|GetWorldLocation (Variables|Default|GetLeftPlate)) (+ LeftHeight (Variables|Default|GetInitialLeft)) _move_to) false false))
        (:then_1
          (Transformation|SetWorldLocation (Variables|Default|GetRightPlate) (Math|Vector|Lerp(Vector) (Transformation|GetWorldLocation (Variables|Default|GetRightPlate)) (+ (Variables|Default|GetInitialRight) RightHeight) _move_to) false false))))))

(event EventBeginPlay
  (Utilities|FlowControl|Sequence
    (:then_0
      (Variables|Default|SetInitialLeft (Transformation|GetWorldLocation (Variables|Default|GetLeftPlate))))
    (:then_1
      (Variables|Default|SetInitialRight (Transformation|GetWorldLocation (Variables|Default|GetRightPlate))))))

(fn ConstructionScript)