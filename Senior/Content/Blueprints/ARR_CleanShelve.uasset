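; ARR_CleanShelve is a proximity trigger, apparently for a clean-shelf interaction, that reacts to Player_BP entering and leaving its overlap area.
; Begin and end overlap set InRange, then share one branch that calls CallButtonTrue or CallButtonFalse accordingly.
; Both branches toggle the Text component's visibility instead of setting it explicitly, so its state depends on the starting visibility.
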(event Collision|EventActorBeginOverlap
  (params (OtherActor :type Actor%20Object%20Reference))
  (Utilities|Casting|CastToPlayer_BP OtherActor)
  (Variables|Default|SetInRange true)
  (if (Variables|Default|GetInRange)
    (Rendering|ToggleVisibility (Variables|Default|GetText) false)
    (Default|CallButtonTrue)
    (else
      (Rendering|ToggleVisibility (Variables|Default|GetText) false)
      (Default|CallButtonFalse))))

(event Collision|EventActorEndOverlap
  (params (OtherActor :type Actor%20Object%20Reference))
  (Utilities|Casting|CastToPlayer_BP OtherActor)
  (Variables|Default|SetInRange false)
  (if (Variables|Default|GetInRange)
    (Rendering|ToggleVisibility (Variables|Default|GetText) false)
    (Default|CallButtonTrue)
    (else
      (Rendering|ToggleVisibility (Variables|Default|GetText) false)
      (Default|CallButtonFalse))))

(fn ConstructionScript)