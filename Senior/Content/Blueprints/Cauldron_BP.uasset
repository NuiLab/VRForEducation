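; Cauldron puzzle actor that collects a red and a blue potion and opens a door once brewed.
; Overlapping actors are matched by first tag; a needed potion is destroyed and sets its colour flag, while CheckObject's display-name check changes nothing.
; HeatUp, not called within this file, requires both flags: the first brew spawns an effect and resets them, later brews spawn another effect and trigger FOR_Door_BP's open event.
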(event Collision|EventActorBeginOverlap
  (params (OtherActor :type Actor%20Object%20Reference))
  (bind _tags (Variables|/Script/Engine.Actor|GetTags OtherActor))
  (bind _output (Utilities|Array|Get(acopy) _tags))
  (bind _returnvalue (Utilities|String|ToString(Name) _output))
  (CallFunction|CheckObject OtherActor)
  (Development|PrintString _returnvalue)
  (bind _destroy (CallFunction|FlagPotion _returnvalue))
  (CallFunction|DeleteObject _destroy OtherActor))

(fn ConstructionScript)

(fn CheckObject
  (params (NewParam :type Actor%20Object%20Reference))
  (bind _returnvalue (Utilities|GetDisplayName NewParam))
  (bind _returnvalue_2 (Utilities|Text|ToText(String) _returnvalue))
  (bind _returnvalue_3 (Utilities|String|ToString(Text) _returnvalue_2))
  (if (Utilities|Enum|Equal(Enum) (Variables|Default|GetpBlue) _returnvalue_3)
    (if (not (Variables|Default|GetpotionBlue))
      (CallFunction|FlagPotion (Variables|Default|GetpBlue)))
    (elif (Utilities|Enum|Equal(Enum) (Variables|Default|GetpRed) _returnvalue_3)
      (if (not (Variables|Default|GetpotionRed))
        (CallFunction|FlagPotion (Variables|Default|GetpRed))))))

(fn FlagPotion
  (params (potion :type String))
  (if (Utilities|Enum|Equal(Enum) potion (Variables|Default|GetpBlue))
    (if (Variables|Default|GetpotionBlue)
      (return false)
      (else
        (return true)))
    (elif (Utilities|Enum|Equal(Enum) potion (Variables|Default|GetpRed))
      (if (Variables|Default|GetpotionRed)
        (return false)
        (else
          (return true)))
      (else
        (return true)))))

(fn DeleteObject
  (params (destroy :type Boolean) (NewParam :type Actor%20Object%20Reference))
  (if destroy
    (if (not (Utilities|Enum|Equal(Enum) (Variables|Default|Getplayer) (Utilities|GetDisplayName NewParam)))
      (if (Utilities|Enum|Equal(Enum) (Variables|Default|GetpBlue) (Utilities|String|ToString(Name) (Utilities|Array|Get(acopy) (Variables|/Script/Engine.Actor|GetTags NewParam))))
        (Actor|DestroyActor NewParam)
        (Variables|Default|SetpotionBlue true)
        (elif (Utilities|Enum|Equal(Enum) (Variables|Default|GetpRed) (Utilities|String|ToString(Name) (Utilities|Array|Get(acopy) (Variables|/Script/Engine.Actor|GetTags NewParam))))
          (Actor|DestroyActor NewParam)
          (Variables|Default|SetpotionRed true))))))

(fn ErrorMsg)

(fn HeatUp
  (bind _c_effect (Variables|Default|GetC_Effect))
  (bind _returnvalue (Transformation|GetSocketLocation _c_effect "None"))
  (if (Variables|Default|GetpotionRed)
    (if (Variables|Default|GetpotionBlue)
      (if (== 0 (Variables|Default|Getcounter))
        (bind _result (Math|Integer|IncrementInt (Variables|Default|Getcounter))
          (:%20%20
            (Variables|Default|Setcounter _result)
            (Variables|Default|SetpotionRed false)
            (Variables|Default|SetpotionBlue false)
            (Effects|SpawnEmitteratLocation "/Game/AlchemistsHouse/P1_Assets/C_Effect_1.C_Effect_1" _returnvalue "0, 0, 0" "1.000000,1.000000,1.000000" false)))
        (elif (== 1 (Variables|Default|Getcounter))
          (Effects|SpawnEmitteratLocation "/Game/AlchemistsHouse/P1_Assets/C_Effect_2.C_Effect_2" _returnvalue)
          (bind _outactors (Actor|GetAllActorsOfClass "/Game/Blueprints/FOR_Door_BP.FOR_Door_BP_C"))
          (Default|OnOpenEvent (Utilities|Array|Get(acopy) _outactors))
          (elif (== 2 (Variables|Default|Getcounter))
            _))))))