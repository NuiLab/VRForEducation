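; Room 3 button Blueprint that reacts to actors entering and leaving its overlap area.
; Begin and end overlap set the IntTrigger flag, then share one branch that toggles the Text component's visibility and calls ButtonTrue on entry or ButtonFalse on exit.
; The overlapping actor is not filtered, and the text is flipped on each event rather than set to match the flag.
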(event Collision|EventActorBeginOverlap
  (params (OtherActor :type Actor%20Object%20Reference))
  (Variables|Default|SetintTrigger true)
  (if (Variables|Default|GetintTrigger)
    (Rendering|ToggleVisibility (Variables|Default|GetText) false)
    (Default|CallButtonTrue)
    (else
      (Rendering|ToggleVisibility (Variables|Default|GetText) false)
      (Default|CallButtonFalse))))

(event Collision|EventActorEndOverlap
  (params (OtherActor :type Actor%20Object%20Reference))
  (Variables|Default|SetintTrigger false)
  (if (Variables|Default|GetintTrigger)
    (Rendering|ToggleVisibility (Variables|Default|GetText) false)
    (Default|CallButtonTrue)
    (else
      (Rendering|ToggleVisibility (Variables|Default|GetText) false)
      (Default|CallButtonFalse))))

(fn ConstructionScript)